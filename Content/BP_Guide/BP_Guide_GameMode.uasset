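; BP_Guide_GameMode is a game mode for a timed statue-collecting game with score, levels and a final rank.
; StartGame resets the state on BeginPlay or RestartGame and starts a looping one-second Clock timer from 30 seconds.
; StatueCollected adds level-scaled score and raises the level every five statues, capped at five, with a zero time bonus.
; At zero, Clock flags game over, calls timer clear with an empty name and assigns a rank by level.
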(event Custom|RestartGame
  ;[1 1 1] Game Start
  (Utilities|StartGame))

(event Custom|Clock
  (Variables|Default|SetTime (- (Variables|Default|GetTime) 1))
  (if (== (Variables|Default|GetTime) 0)
    (Variables|Default|SetGameOver true)
    (Utilities|Time|ClearTimerbyFunctionName 0 "")
    (switch int (Variables|Default|GetLevel)
      (:1
        (Variables|Default|SetRank "Rookie"))
      (:2
        (Variables|Default|SetRank "Bronze"))
      (:3
        (Variables|Default|SetRank "Silver"))
      (:4
        (Variables|Default|SetRank "Gold"))
      (:5
        (Variables|Default|SetRank "Diamond")))))

(event EventBeginPlay
  ;[1 1 1] Game Start
  (Utilities|StartGame))

(fn ConstructionScript)

(fn StatueCollected
  ;[1 1 1] Statue
  (Variables|Default|SetScore (+ (Variables|Default|GetScore) (* (Variables|Default|GetLevel) 10)))
  (Variables|Default|SetStatueCount (+ (Variables|Default|GetStatueCount) 1))
  (if (== (Math|Integer|%(Integer) (Variables|Default|GetStatueCount) 5) 0)
    (Variables|Default|SetTime (+ (Variables|Default|GetTime) 0))
    (Variables|Default|SetLevel (Math|Integer|Min(Integer) (+ (Variables|Default|GetLevel) 1) 5))))