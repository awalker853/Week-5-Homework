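; HUD class for the Guide game that shows score, time, player level and the game-over screen.
; On BeginPlay it casts the game mode to BP_Guide_GameMode and caches it.
; DrawHUD draws text each frame at fixed screen positions from that game mode's values.
; When GameOver is set, it adds a game over message, a Press Enter prompt and the rank.
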(event EventBeginPlay
  (bind _asbp_guide_game_mode (Utilities|Casting|CastToBP_Guide_GameMode (Game|GetGameMode)))
  (Variables|Default|SetMy_Guide_GameMode _asbp_guide_game_mode))

(event EventDrawHUD
  (params (SizeX :type Integer) (SizeY :type Integer))
  (HUD|DrawText (Utilities|String|BuildString(Integer) "Score" "" (Variables|/Game/BP_Guide/BP_Guide_GameMode.BP_Guide_GameMode_C|GetScore (Variables|Default|GetMy_Guide_GameMode))) "(R=0.979167,G=0.860294,B=0.030599,A=1.000000)" 1e+01 1e+01 0 3.0 false)
  (HUD|DrawText (Utilities|String|BuildString(Integer) "Time" "" (Variables|/Game/BP_Guide/BP_Guide_GameMode.BP_Guide_GameMode_C|GetTime (Variables|Default|GetMy_Guide_GameMode))) "(R=1.000000,G=0.000000,B=0.008024,A=1.000000)" 3e+02 1e+01 0 3.0 false)
  (HUD|DrawText (Utilities|String|BuildString(Integer) "Player Level:" "" (Variables|/Game/BP_Guide/BP_Guide_GameMode.BP_Guide_GameMode_C|GetLevel (Variables|Default|GetMy_Guide_GameMode))) "(R=0.000000,G=0.109471,B=0.416667,A=1.000000)" 5.5e+02 1e+01 0 3.0 false)
  (if (Variables|/Game/BP_Guide/BP_Guide_GameMode.BP_Guide_GameMode_C|GetGameOver (Variables|Default|GetMy_Guide_GameMode))
    (HUD|DrawText "GAME OVER" "(R=0.947917,G=0.044434,B=0.044434,A=1.000000)" 4e+02 2e+02 0 3.0 false)
    (HUD|DrawText "Press Enter" "(R=0.838542,G=0.131022,B=0.131022,A=1.000000)" 4e+02 4e+02 0 3.0 false)
    (HUD|DrawText (Utilities|String|Append "Rank:" (Variables|/Game/BP_Guide/BP_Guide_GameMode.BP_Guide_GameMode_C|GetRank (Variables|Default|GetMy_Guide_GameMode))) "(R=1.000000,G=0.000000,B=0.000000,A=1.000000)" 4e+02 3e+02 0 3.0 false)))

(fn ConstructionScript)