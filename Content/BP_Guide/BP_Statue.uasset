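; BP_Statue is a collectible that jumps around the level for the player to catch.
; InitStatue teleports it to a random point in a square around the world origin, then re-arms itself on a timer that shortens as the GameMode's Level rises.
; When the player overlaps it before game over, it notifies BP_Guide_GameMode, destroys itself and spawns a replacement, which relocates on BeginPlay.
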(event EventBeginPlay
  (bind _asbp_guide_game_mode (Utilities|Casting|CastToBP_Guide_GameMode (Game|GetGameMode)))
  (Variables|Default|SetBP_Guide_GameMode _asbp_guide_game_mode)
  (CallFunction|InitStatue))

(event Collision|EventActorBeginOverlap
  (params (OtherActor :type Actor%20Object%20Reference))
  (if (and (== OtherActor (Game|GetPlayerCharacter 0)) (not (Variables|/Game/BP_Guide/BP_Guide_GameMode.BP_Guide_GameMode_C|GetGameOver (Variables|Default|GetBP_Guide_GameMode))))
    (Default|StatueCollected (Variables|Default|GetBP_Guide_GameMode))
    (Actor|DestroyActor)
    (Game|SpawnActorfromClass "BP_Statue_C" (Transformation|GetActorTransform) "Undefined" 0 0)))

(fn ConstructionScript)

(fn InitStatue
  (Transformation|Teleport (Math|Vector|MakeVector (Math|Random|RandomFloatinRange -1e+03 1e+03) (Math|Random|RandomFloatinRange -1e+03 1e+03) 5e+01) "0, 0, 0")
  (Utilities|Time|SetTimerbyFunctionName 0 "InitStatue" (Math|Conversions|ToFloat(Integer) (- 6 (Variables|/Game/BP_Guide/BP_Guide_GameMode.BP_Guide_GameMode_C|GetLevel (Variables|Default|GetBP_Guide_GameMode))))))